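; WaterFall gameplay ability for the Aura character that fires a projectile toward where the camera is looking when the input is released.
; On release it projects a target point along the camera's forward vector by Range, without a trace, and updates the character's facing target.
; The cast montage's gameplay event then triggers the projectile spawn from the right-hand socket, and the ability commits only afterward before ending.
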(event `self.K2_ActivateAbility`
  (`AbilityTask_WaitInputRelease.WaitInputRelease` false
    (:`OnRelease`
      (`self.SetTargetLocation`)
      (`AbilityTask_PlayMontageAndWait.CreatePlayMontageAndWaitProxy` "None" "/Game/Assets/Characters/Aura/Animations/Abilities/AM_Cast_WaterFall.AM_Cast_WaterFall" 1.0 "None" false
        (:`then`
          (`AbilityTask_WaitGameplayEvent.WaitGameplayEvent` (struct :`TagName` "Event.Montage.WaterFall") null
            (:`EventReceived`
              (`self.SpawnProjectile` (`self.ProjectileTargetLocation`) (`BlueprintGameplayTagLibrary.MakeLiteralGameplayTag` (struct :`TagName` "CombatSocket.RightHand")))
              (`self.K2_CommitAbility`)
              (`self.K2_EndAbility`))))))))

(fn `SetTargetLocation`
  (locals (LocalOutHit :type "HitResult Structure"))
  (`KismetArrayLibrary.Array_Clear` (`self.ActorsIgnore`))
  (bind _asbp_aura_character (cast `/Game/Blueprints/Character/Aura/BP_AuraCharacter` (`self.GetAvatarActorFromActorInfo`)))
  (bind _output_get (set `self.BPAuraCharacter` _asbp_aura_character))
  (bind _returnvalue (`AuraCharacter.GetCameraComponent` _output_get))
  (bind _returnvalue_2 (`SceneComponent.GetForwardVector` _returnvalue))
  (set `self.Direction` _returnvalue_2)
  (bind _output_get_2 (set `self.ProjectileTargetLocation` (+ (`SceneComponent.K2_GetComponentLocation` _returnvalue) (* _returnvalue_2 (`self.Range`)))))
  (message `CombatInterface.UpdateFacingTarget` (`self.BPAuraCharacter`) _output_get_2)
  (return))