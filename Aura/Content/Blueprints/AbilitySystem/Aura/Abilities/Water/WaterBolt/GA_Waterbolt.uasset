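; Water Bolt gameplay ability for the Aura character that fires water projectiles from the weapon socket when input is released.
; A sphere trace from the weapon toward a point along the camera's forward vector sets the target location and stores hit BP_BaseTree actors.
; A cast montage's gameplay event spawns homing spread projectiles if a stored actor is valid, otherwise a single projectile.
; The ability commits only after spawning, then ends.
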(event `self.K2_ActivateAbility`
  (`AbilityTask_WaitInputRelease.WaitInputRelease` false
    (:`OnRelease`
      (`self.SetTargetLocationAndHitActor`)
      (`/Engine/EditorBlueprintResources/StandardMacros.IsValid` (`self.MouseHitActor`)
        (:`Is Valid`
          (`AbilityTask_PlayMontageAndWait.CreatePlayMontageAndWaitProxy` "None" "/Game/Assets/Characters/Aura/Animations/Abilities/AM_Cast_WaterBolt.AM_Cast_WaterBolt" 1.0 "None" false
            (:`then`
              (`AbilityTask_WaitGameplayEvent.WaitGameplayEvent` (struct :`TagName` "Event.Montage.Waterbolt") null
                (:`EventReceived`
                  (`self.SpawnSpreadProjectiles` (`self.ProjectileTargetLocation`) (`BlueprintGameplayTagLibrary.MakeLiteralGameplayTag` (struct :`TagName` "CombatSocket.Weapon")) false 25.0 (`self.MouseHitActor`)))))))
        (:`Is Not Valid`
          (`AbilityTask_PlayMontageAndWait.CreatePlayMontageAndWaitProxy` "None" "/Game/Assets/Characters/Aura/Animations/Abilities/AM_Cast_WaterBolt.AM_Cast_WaterBolt" 1.0 "None" false
            (:`then`
              (`AbilityTask_WaitGameplayEvent.WaitGameplayEvent` (struct :`TagName` "Event.Montage.Waterbolt") null
                (:`EventReceived`
                  (`self.SpawnProjectile` (`self.ProjectileTargetLocation`) (`BlueprintGameplayTagLibrary.MakeLiteralGameplayTag` (struct :`TagName` "CombatSocket.Weapon")))))))))
      (`self.K2_CommitAbility`)
      (`self.K2_EndAbility`))))

(fn `SetTargetLocationAndHitActor`
  (locals (LocalOutHit :type "HitResult Structure"))
  (bind _actorsignore (`self.ActorsIgnore`))
  (`KismetArrayLibrary.Array_Clear` (`self.ActorsIgnore`))
  (bind _asbp_aura_character (cast `/Game/Blueprints/Character/Aura/BP_AuraCharacter` (`self.GetAvatarActorFromActorInfo`)))
  (bind _output_get (set `self.BPAuraCharacter` _asbp_aura_character))
  (bind _returnvalue (`AuraCharacter.GetCameraComponent` _output_get))
  (bind _returnvalue_2 (message `CombatInterface.GetCombatSocketLocation` (`self.BPAuraCharacter`) (`BlueprintGameplayTagLibrary.MakeLiteralGameplayTag` (struct :`TagName` "CombatSocket.Weapon"))))
  (message `CombatInterface.GetWeapon` (`self.BPAuraCharacter`))
  (`KismetArrayLibrary.Array_AddUnique` _actorsignore)
  (`KismetArrayLibrary.Array_AddUnique` _actorsignore (`self.BPAuraCharacter`))
  (bind _returnvalue_3 (+ (`SceneComponent.K2_GetComponentLocation` _returnvalue) (* (`SceneComponent.GetForwardVector` _returnvalue) (`self.Range`))))
  (bind (_outhit _returnvalue_4) (`KismetSystemLibrary.SphereTraceSingleByProfile` _returnvalue_2 _returnvalue_3 10.0 "OverlapOnlyPawn" false (`self.ActorsIgnore`) "None" true (struct :`R` 1.0 :`A` 1.0) (struct :`G` 1.0 :`A` 1.0) 10.0))
  (if _returnvalue_4
    (bind _output_get_2 (set `local.LocalOutHit` _outhit))
    (set `self.ProjectileTargetLocation` (`.ImpactPoint` (`GameplayStatics.BreakHitResult` _output_get_2)))
    (cast `/Game/Blueprints/Actor/Tree/BP_BaseTree` (`.HitActor` (`GameplayStatics.BreakHitResult` _output_get_2))
      (:`then`
        (bind _output_get_3 (set `self.MouseHitActor` (`.HitActor` (`GameplayStatics.BreakHitResult` _output_get_2))))
        (`/Engine/EditorBlueprintResources/StandardMacros.IsValid` _output_get_3
          (:`Is Valid`
            (message `CombatInterface.UpdateFacingTarget` (`self.BPAuraCharacter`) (`Actor.K2_GetActorLocation` _output_get_3))
            (return))
          (:`Is Not Valid`
            _)))
      (:`CastFailed`
        _))
    (return)
    (else
      (set `self.MouseHitActor` null)
      (bind _output_get_4 (set `self.ProjectileTargetLocation` _returnvalue_3))
      (message `CombatInterface.UpdateFacingTarget` (`self.BPAuraCharacter`) _output_get_4)
      (return))))