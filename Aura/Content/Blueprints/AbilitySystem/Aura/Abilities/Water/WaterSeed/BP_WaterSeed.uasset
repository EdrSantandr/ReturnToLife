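; Water Seed ability actor that plants a small forest where it overlaps the landscape, then explodes and destroys itself.
; On impact it queries actors within the forest radius for toxic terrain.
; Clean ground gets random trees, rolled per saved billboard marker and dropped to the surface by a downward line trace.
; Toxic ground instead pauses the game and shows an info widget with UI-only input.
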(event `self.ReceiveBeginPlay`
  (`self.SaveBillboardComponents`))

(event `self.SphereComponent.OnComponentBeginOverlap`
  (params (OverlappedComponent :type "PrimitiveComponent Object Reference") (OtherActor :type "Actor Object Reference") (OtherComp :type "PrimitiveComponent Object Reference") (OtherBodyIndex :type Integer) (bFromSweep :type Boolean) (SweepResult :type "HitResult Structure (by ref)"))
  (cast `Landscape` OtherActor)
  (`KismetArrayLibrary.Array_AddUnique` (`self.ActorsIgnore`) self)
  (bind _outoverlappedactors (`AuraAbilitySystemLibrary.GetLiveTreesWithinRadius` self (`self.ActorsIgnore`) (`self.ForestAreaRadius`) (`self.K2_GetActorLocation`)))
  (bind _result (`self.CheckTerrain` _outoverlappedactors))
  (if _result
    (`KismetSystemLibrary.PrintString` "Clean terrain")
    (`self.PlantTrees`)
    (else
      (`self.ShowInfoWidget`)))
  (`NiagaraFunctionLibrary.SpawnSystemAtLocation` (`self.ExplodeSystem`) (`self.K2_GetActorLocation`))
  (`self.K2_DestroyActor`))

(fn `CheckTerrain`
  (params (InActors :type "Array of Actor Object Reference"))
  (returns (Result :type Boolean))
  (for _array_element InActors
    (cast `/Game/Blueprints/Actor/Tree/BP_BaseToxicTerrain` _array_element)
    (return false))
  (return true))

(fn `GetFixedTreeLocation`
  (params (InLocation :type "Vector Structure"))
  (returns (OutLocation :type "Vector Structure"))
  (locals (DistanceToCheck :type "Float (double-precision)" :default 600.0))
  (bind (_outhit _returnvalue) (`KismetSystemLibrary.LineTraceSingleByProfile` :`Start` InLocation :`End` (+ InLocation (* (`KismetMathLibrary.Vector_Down`) (`local.DistanceToCheck`))) :`ProfileName` "BlockAll" :`DrawTime` 6.0))
  (if _returnvalue
    (return (`.ImpactPoint` (`GameplayStatics.BreakHitResult` _outhit)))
    (else
      (return (0.0 0.0 0.0)))))

(fn `PlantTrees`
  (for _array_element (`self.BillboardComponents`)
    (if (<= (`KismetMathLibrary.RandomFloatInRange` 0.0 1.0) (`self.TreeChance`))
      (bind _outlocation (`self.GetFixedTreeLocation` (`SceneComponent.K2_GetComponentLocation` _array_element)))
      (`|SpawnActorFromClass` (`KismetArrayLibrary.Array_Random` (`self.ArrayTrees`)) (`KismetMathLibrary.MakeTransform` _outlocation) "AdjustIfPossibleButAlwaysSpawn" "MultiplyWithRoot" null null)))
  (return))

(fn `SaveBillboardComponents`
  (`KismetArrayLibrary.Array_AddUnique` (`self.BillboardComponents`) (`self.Bill9`))
  (`KismetArrayLibrary.Array_AddUnique` (`self.BillboardComponents`) (`self.Bill8`))
  (`KismetArrayLibrary.Array_AddUnique` (`self.BillboardComponents`) (`self.Bill7`))
  (`KismetArrayLibrary.Array_AddUnique` (`self.BillboardComponents`) (`self.Bill6`))
  (`KismetArrayLibrary.Array_AddUnique` (`self.BillboardComponents`) (`self.Bill5`))
  (`KismetArrayLibrary.Array_AddUnique` (`self.BillboardComponents`) (`self.Bill4`))
  (`KismetArrayLibrary.Array_AddUnique` (`self.BillboardComponents`) (`self.Bill3`))
  (`KismetArrayLibrary.Array_AddUnique` (`self.BillboardComponents`) (`self.Bill2`))
  (`KismetArrayLibrary.Array_AddUnique` (`self.BillboardComponents`) (`self.Bill1`)))

(fn `ShowInfoWidget`
  (bind _returnvalue (`GameplayStatics.GetPlayerController` 0))
  (set `PlayerController.bShowMouseCursor` true _returnvalue)
  (`WidgetBlueprintLibrary.SetInputMode_UIOnlyEx` _returnvalue null)
  (bind _returnvalue_2 (`|CreateWidget` "/Game/Blueprints/UI/Info/WBP_CanvasInfo.WBP_CanvasInfo_C"))
  (`UserWidget.AddToViewport` _returnvalue_2 0)
  (`GameplayStatics.SetGamePaused` true))

(fn `UserConstructionScript`)