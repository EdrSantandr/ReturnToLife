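; Water Purify ability actor that grows in place and cleanses toxic terrain around it.
; On BeginPlay it deactivates its projectile movement and plays a timeline that scales it up toward FinalScale.
; When the timeline finishes, it queries GetLiveTreesWithinRadius using the scaled sphere radius, ignoring itself and its owner, and calls Purify on BP_BaseToxicTerrain results.
; It destroys itself after a short delay.
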(event `self.ReceiveBeginPlay`
  (bind _actorsignore (`self.ActorsIgnore`))
  (`KismetArrayLibrary.Array_AddUnique` _actorsignore self)
  (`KismetArrayLibrary.Array_AddUnique` _actorsignore (`self.GetOwner`))
  (`ActorComponent.Deactivate` (`self.ProjectileMovementComponent`))
  (bind (_direction _scale) (`Timeline|Initial`)
    (:`Update`
      (`self.SetActorScale3D` (`KismetMathLibrary.Conv_DoubleToVector` (* _scale (`self.FinalScale`)))))
    (:`Finished`
      (bind _outoverlappedactors (`AuraAbilitySystemLibrary.GetLiveTreesWithinRadius` self (`self.ActorsIgnore`) (* (`SphereComponent.SphereRadius` (`self.SphereComponent`)) (`self.FinalScale`)) (`self.K2_GetActorLocation`)))
      (for _array_element _outoverlappedactors
        (bind _asbp_base_toxic_terrain (cast `/Game/Blueprints/Actor/Tree/BP_BaseToxicTerrain` _array_element))
        (`/Game/Blueprints/Actor/Tree/BP_BaseToxicTerrain.Purify` _asbp_base_toxic_terrain))
      (`KismetSystemLibrary.Delay` 0.5)
      (`self.K2_DestroyActor`))))

(fn `UserConstructionScript`)