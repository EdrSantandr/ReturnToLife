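; BP_WaterRain is a water ability actor that extinguishes burning trees through BP_BaseTree's DeBurn.
; It enables query-only sphere collision shortly after spawning; overlapping a tree calls DeBurn, plays impact sound and water explosion, then destroys itself.
; Tick watches its height and, once it has risen MaxHeight above its starting Z, spawns a configurable actor class with a water explosion and destroys itself.
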(event `self.ReceiveBeginPlay`
  (bind (_returnvalue_x _returnvalue_y _returnvalue_z) (`KismetMathLibrary.BreakVector` (`self.K2_GetActorLocation`)))
  (set `self.InitialZ` _returnvalue_z)
  (`KismetSystemLibrary.Delay` 0.1)
  (bind _spherecomponent (`self.SphereComponent`)
    (:`then`
      (`PrimitiveComponent.SetCollisionEnabled` _spherecomponent "QueryOnly"))
    (:`else`)))

(event `self.ReceiveTick`
  (params (DeltaSeconds :type "Float (single-precision)"))
  (bind (_returnvalue_x _returnvalue_y _returnvalue_z) (`KismetMathLibrary.BreakVector` (`self.K2_GetActorLocation`)))
  (if (<= (+ (`self.InitialZ`) (`self.MaxHeight`)) _returnvalue_z)
    (`|SpawnActorFromClass` (`self.Class`) (`KismetMathLibrary.MakeTransform` (`self.K2_GetActorLocation`)) "Undefined" "MultiplyWithRoot" null null)
    (`NiagaraFunctionLibrary.SpawnSystemAtLocation` "/Game/Assets/Effects/Projectiles/FireExplosion/NS_WaterExplosion.NS_WaterExplosion" (`self.K2_GetActorLocation`))
    (`self.K2_DestroyActor`)))

(event `self.SphereComponent.OnComponentBeginOverlap`
  (params (OverlappedComponent :type "PrimitiveComponent Object Reference") (OtherActor :type "Actor Object Reference") (OtherComp :type "PrimitiveComponent Object Reference") (OtherBodyIndex :type Integer) (bFromSweep :type Boolean) (SweepResult :type "HitResult Structure (by ref)"))
  (bind _returnvalue (`self.K2_GetActorLocation`))
  (bind _asbp_base_tree (cast `/Game/Blueprints/Actor/Tree/BP_BaseTree` OtherActor))
  (bind _output_get (set `self.CollidedBaseTree` _asbp_base_tree))
  (`/Game/Blueprints/Actor/Tree/BP_BaseTree.DeBurn` _output_get)
  (`GameplayStatics.SpawnSoundAtLocation` "/Game/Assets/Sounds/Abilities/FireBolt/sfx_FireBolt_Impact.sfx_FireBolt_Impact" _returnvalue (struct) 1.0 1.0 0.0 null null)
  (`NiagaraFunctionLibrary.SpawnSystemAtLocation` "/Game/Assets/Effects/Projectiles/FireExplosion/NS_WaterExplosion.NS_WaterExplosion" _returnvalue)
  (`self.K2_DestroyActor`))

(fn `UserConstructionScript`)