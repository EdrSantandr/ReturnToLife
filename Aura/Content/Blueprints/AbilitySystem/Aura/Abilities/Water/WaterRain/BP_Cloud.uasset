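; Rain cloud actor for the Water Rain ability that fires homing waterbolts at live trees within its effect radius.
; On BeginPlay it gathers target trees once and starts a looping timer.
; Each tick of the timer launches a BP_Waterbolt from one of four random spawn points, homing on a random tree.
; The cloud destroys itself once the spawn limit is reached, counting attempts without a valid target.
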(event `self.ReceiveBeginPlay`
  (bind _spawnlocations (`self.SpawnLocations`))
  (set `self.ProjectilesSpawned` 0)
  (`KismetArrayLibrary.Array_AddUnique` _spawnlocations (`self.Bill1`))
  (`KismetArrayLibrary.Array_AddUnique` _spawnlocations (`self.Bill2`))
  (`KismetArrayLibrary.Array_AddUnique` _spawnlocations (`self.Bill3`))
  (`KismetArrayLibrary.Array_AddUnique` _spawnlocations (`self.Bill4`))
  (`KismetArrayLibrary.Array_AddUnique` (`self.Actors to Ignore`) self)
  (bind _outoverlappedactors (`AuraAbilitySystemLibrary.GetLiveTreesWithinRadius` self (`self.Actors to Ignore`) (`self.CloudEffectRadius`) (`self.K2_GetActorLocation`)))
  (set `self.HomingTargets` _outoverlappedactors)
  (bind _returnvalue (`KismetSystemLibrary.K2_SetTimerDelegate` (delegate `SpawnProjectiles`) 0.5 true))
  (set `self.SpawnTimerHandle` _returnvalue))

(event `SpawnProjectiles`
  (if (<= (`self.MaxProjectilesSpawned`) (`self.ProjectilesSpawned`))
    (`KismetSystemLibrary.K2_ClearAndInvalidateTimerHandle` (`self.SpawnTimerHandle`))
    (`self.K2_DestroyActor`)
    (else
      (`self.SpawnCloudProjectile`))))

(fn `GetRandomHomingTarget`
  (returns (OutHomingTarget :type "Actor Object Reference"))
  (bind _homingtargets (`self.HomingTargets`))
  (return (`|GetArrayItem` _homingtargets (`KismetMathLibrary.RandomIntegerInRange` 0 (- (`KismetArrayLibrary.Array_Length` _homingtargets) 1)))))

(fn `SpawnCloudProjectile`
  (bind _spawnlocations (`self.SpawnLocations`))
  (bind _returnvalue (`SceneComponent.K2_GetComponentLocation` (`|GetArrayItem` _spawnlocations (`KismetMathLibrary.RandomIntegerInRange` 0 (- (`KismetArrayLibrary.Array_Length` _spawnlocations) 1)))))
  (`/Engine/EditorBlueprintResources/StandardMacros.IncrementInt` (`self.ProjectilesSpawned`)
    (:`  `
      (bind _outhomingtarget (`self.GetRandomHomingTarget`))
      (`/Engine/EditorBlueprintResources/StandardMacros.IsValid` _outhomingtarget
        (:`Is Valid`
          (bind _returnvalue_2 (`|SpawnActorFromClass` (`self.Class`) (`KismetMathLibrary.MakeTransform` _returnvalue (`KismetMathLibrary.FindLookAtRotation` _returnvalue (`self.K2_GetActorLocation` _outhomingtarget))) "AdjustIfPossibleButAlwaysSpawn" "MultiplyWithRoot" self null))
          (bind _asbp_waterbolt (cast `/Game/Blueprints/AbilitySystem/Aura/Abilities/Water/WaterBolt/BP_Waterbolt` _returnvalue_2))
          (bind _projectilemovementcomponent (`AuraProjectile.ProjectileMovementComponent` _asbp_waterbolt))
          (set `ProjectileMovementComponent.HomingTargetComponent` (`self.GetComponentByClass` _outhomingtarget "/Script/Engine.SceneComponent") _projectilemovementcomponent)
          (set `ProjectileMovementComponent.bIsHomingProjectile` true _projectilemovementcomponent))))))

(fn `UserConstructionScript`)