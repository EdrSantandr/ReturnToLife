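; Firebolt gameplay ability that auto-attacks the highlighted actor under the mouse with homing spread projectiles.
; On activation it checks target and range, faces the target and starts a looping attack timer, otherwise it ends, with a message if out of range.
; Each tick re-faces the target, plays the cast montage and spawns projectiles on its gameplay event.
; Pressing input again or a dead or non-combat target clears the timer and ends the ability.
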(event `self.K2_ActivateAbility`
  (`KismetSystemLibrary.PrintString` "firebolt")
  (`TargetDataUnderMouse.CreateTargetDataUnderMouse`
    (:`MouseTargetDataSignature`
      (bind _returnvalue (`AuraAbilitySystemLibrary.GetHighLightedActor` null))
      (`/Engine/EditorBlueprintResources/StandardMacros.IsValid` _returnvalue
        (:`Is Valid`
          (bind _output_get (set `self.MouseHitActor` _returnvalue))
          (bind _output_get_2 (set `self.ProjectileTargetLocation` (`Actor.K2_GetActorLocation` _output_get)))
          (bind _returnvalue_2 (`self.CheckAbilityRange` _output_get_2))
          (if _returnvalue_2
            (message `CombatInterface.UpdateFacingTarget` (`self.GetAvatarActorFromActorInfo`) (`self.ProjectileTargetLocation`))
            (bind _returnvalue_3 (`KismetSystemLibrary.K2_SetTimerDelegate` (delegate `AutoAttack`) (`self.AutoAttackDeltaTime`) true false -0.4))
            (set `self.AutoAttackTimerHandle` _returnvalue_3)
            (else
              (`self.SendMessageBP` (`BlueprintGameplayTagLibrary.MakeLiteralGameplayTag` (struct :`TagName` "Message.TargetOutOfRange")))
              (`self.K2_EndAbility` :!label _label))))
        (:`Is Not Valid`
          (goto _label))))))

(event `AutoAttack`
  (bind _mousehitactor (`self.MouseHitActor`))
  (`AbilityTask_WaitInputPress.WaitInputPress` false
    (:`then`
      (if (`KismetSystemLibrary.DoesImplementInterface` _mousehitactor "/Script/Aura.CombatInterface")
        (bind _returnvalue (message `CombatInterface.IsDead` _mousehitactor))
        (if (not _returnvalue)
          (message `CombatInterface.UpdateFacingTarget` (`self.GetAvatarActorFromActorInfo`) (`Actor.K2_GetActorLocation` (`self.MouseHitActor`)))
          (`AbilityTask_PlayMontageAndWait.CreatePlayMontageAndWaitProxy` "None" "/Game/Assets/Characters/Aura/Animations/Abilities/AM_Cast_FireBolt.AM_Cast_FireBolt" 1.0 "None" false
            (:`then`
              (`AbilityTask_WaitGameplayEvent.WaitGameplayEvent` (struct :`TagName` "Event.Montage.Firebolt") null
                (:`EventReceived`
                  (`self.SpawnSpreadProjectiles` (`self.ProjectileTargetLocation`) (`BlueprintGameplayTagLibrary.MakeLiteralGameplayTag` (struct :`TagName` "CombatSocket.Weapon")) true 25.0 (`self.MouseHitActor`))))))
          (else
            (`self.PrepareToEnd` :!label _label_2)
            (`self.K2_EndAbility`)))
        (else
          (goto _label_2))))
    (:`OnPress`
      (goto _label_2))))

(fn `PrepareToEnd`
  (set `self.MouseHitActor` null)
  (`KismetSystemLibrary.K2_ClearAndInvalidateTimerHandle` (`self.AutoAttackTimerHandle`)))