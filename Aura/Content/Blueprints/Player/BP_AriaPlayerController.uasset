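; Player controller Blueprint that handles camera zoom and crosshair display for the possessed AuraCharacter.
; BeginPlay caches the character, its camera and the overlay widget from BP_AuraHUD, then hides the crosshair.
; CameraZoomin shows the crosshair and plays a timeline that narrows the camera's field of view.
; CameraZoomOut hides the crosshair and reverses that same timeline to restore the view.
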(event `self.ReceiveBeginPlay`
  (bind _asaura_character (cast `AuraCharacter` (`self.K2_GetPawn`)))
  (bind _output_get (set `self.AuraCharacter` _asaura_character))
  (bind _returnvalue (`AuraCharacter.GetCameraComponent` _output_get))
  (set `self.PlayerCamera` _returnvalue)
  (bind _asbp_aura_hud (cast `/Game/Blueprints/UI/HUD/BP_AuraHUD` (`self.GetHUD`)))
  (bind _output_get_2 (set `self.BPAuraHUD` _asbp_aura_hud))
  (bind _returnvalue_2 (`AuraHUD.GetOverlayWidget` _output_get_2))
  (bind _aswbp_overlay (cast `/Game/Blueprints/UI/Overlay/WBP_Overlay` _returnvalue_2))
  (bind _output_get_3 (set `self.WBPOverlay` _aswbp_overlay))
  (`/Game/Blueprints/UI/Overlay/WBP_Overlay.EnableCrosshair` _output_get_3 false))

(event `self.CameraZoomIn`
  (`/Engine/EditorBlueprintResources/StandardMacros.IsValid` (`self.AuraCharacter`)
    (:`Is Valid`
      (`/Game/Blueprints/UI/Overlay/WBP_Overlay.EnableCrosshair` (`self.WBPOverlay`) true)
      (bind (_direction _zoom) (`Timeline|ZoomTimeline` :!label _label)
        (:`Update`
          (`CameraComponent.SetFieldOfView` (`self.PlayerCamera`) (`KismetMathLibrary.Lerp` 90.0 60.0 _zoom)))))))

(event `self.CameraZoomOut`
  (`/Engine/EditorBlueprintResources/StandardMacros.IsValid` (`self.AuraCharacter`)
    (:`Is Valid`
      (`/Game/Blueprints/UI/Overlay/WBP_Overlay.EnableCrosshair` (`self.WBPOverlay`) false)
      (goto _label :!via `Reverse`))))

(fn `UserConstructionScript`)