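; Base toxic terrain actor that can be detected and purified.
; Detection activates a Niagara effect for a set duration, then deactivates it.
; Purify uses a timeline to raise the level's directional light intensity by up to one unit, then reports itself to BP_AriaGameMode's toxicity check and destroys itself.
; Purification only proceeds if a directional light exists in the level.
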(event `Detected`
  (bind _detectedniagara (`self.DetectedNiagara`))
  (`ActorComponent.Activate` _detectedniagara true)
  (`KismetSystemLibrary.Delay` (`self.TimeDetected`))
  (`ActorComponent.Deactivate` _detectedniagara))

(event `Purify`
  (bind _initialintensity (`self.InitialIntensity`))
  (bind _returnvalue (`GameplayStatics.GetActorOfClass` "/Script/Engine.DirectionalLight"))
  (`/Engine/EditorBlueprintResources/StandardMacros.IsValid` _returnvalue
    (:`Is Valid`
      (bind _output_get (set `self.DirectionalLight` _returnvalue))
      (set `self.InitialIntensity` (`LightComponentBase.Intensity` (`Light.LightComponent` _output_get)))
      (bind (_direction _intensity) (`Timeline|LightTimeline`)
        (:`Update`
          (`LightComponent.SetIntensity` (`Light.LightComponent` (`self.DirectionalLight`)) (`KismetMathLibrary.Lerp` _initialintensity (+ _initialintensity 1.0) _intensity)))
        (:`Finished`
          (`self.RemoveFromGame`)
          (`self.K2_DestroyActor`))))))

(fn `RemoveFromGame`
  (bind _asbp_aria_game_mode (cast `/Game/Blueprints/Game/BP_AriaGameMode` (`GameplayStatics.GetGameMode`)))
  (`/Game/Blueprints/Game/BP_AriaGameMode.VerifyToxicity` _asbp_aria_game_mode self))

(fn `UserConstructionScript`)