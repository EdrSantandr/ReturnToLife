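; BP_TreeChild is a tree actor that animates its own appearance when play begins.
; It first raises itself by its capsule half-height, then plays a timeline that drives uniform scale and adds yaw each update, multiplied by a per-instance random factor.
; When the timeline finishes, it spawns a Niagara effect at the actor's location.
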(event `self.ReceiveBeginPlay`
  (bind _output_get (set `self.CapsuleHeight` (`CapsuleComponent.CapsuleHalfHeight` (`self.Capsule`))))
  (bind _output_get_2 (set `self.InitialLocation` (`self.K2_GetActorLocation`)))
  (`self.K2_SetActorLocation` (`KismetMathLibrary.MakeVector` (.x _output_get_2) (.y _output_get_2) (+ (.z _output_get_2) _output_get)))
  (set `self.RandomRotation` (`KismetMathLibrary.RandomFloatInRange` 0.0 6.0))
  (bind (_direction _scale _rotation) (`Timeline|ScaleTimeline`)
    (:`Update`
      (`self.SetActorScale3D` (`KismetMathLibrary.Conv_DoubleToVector` _scale))
      (`self.K2_AddActorLocalRotation` (`KismetMathLibrary.MakeRotator` 0.0 0.0 (* _rotation (`self.RandomRotation`)))))
    (:`Finished`
      (`NiagaraFunctionLibrary.SpawnSystemAtLocation` (`self.NiagaraTreeSpawned`) (`self.K2_GetActorLocation`)))))

(fn `UserConstructionScript`
  (`parent.UserConstructionScript`))