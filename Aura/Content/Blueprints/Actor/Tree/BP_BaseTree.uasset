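; Base tree actor that can randomly catch fire at BeginPlay, burn for a random lifespan, and play cracking sound and VFX when destroyed.
; Burning trees tick at randomized intervals, passing live trees within FireRadius to Burn, whose guard tests the caller's IsBurning rather than the target's.
; Burn rolls ChanceToBurn before enabling fire, tick and lifespan.
; DeBurn stops the fire, clears the lifespan and spawns a heal effect.
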(event `self.ReceiveBeginPlay`
  (`self.SetActorTickInterval` (`KismetMathLibrary.RandomFloatInRange` 3.0 6.0))
  (`self.Burn` self)
  (add `self.OnDestroyed` (delegate `OnDestroyed_Event`)))

(event `OnDestroyed_Event` :!signature `self.OnDestroyed`
  (params (DestroyedActor :type "Actor Object Reference"))
  (bind _returnvalue (`self.K2_GetActorLocation` DestroyedActor))
  (`GameplayStatics.SpawnSoundAtLocation` "/Game/Assets/Sounds/Effects/SE_WoodCracking.SE_WoodCracking" _returnvalue (struct) 1.0 1.0 0.0 null null)
  (`NiagaraFunctionLibrary.SpawnSystemAtLocation` (`self.DeadVFX`) _returnvalue))

(event `self.ReceiveTick`
  (params (DeltaSeconds :type "Float (single-precision)"))
  (if (`self.bIsBurning`)
    (`self.SetActorTickInterval` (`KismetMathLibrary.RandomFloatInRange` 6.0 8.0))
    (`KismetArrayLibrary.Array_AddUnique` (`self.ActorsToIgnore`) self)
    (bind _outoverlappedactors (`AuraAbilitySystemLibrary.GetLiveTreesWithinRadius` self (`self.ActorsToIgnore`) (`self.FireRadius`) (`self.K2_GetActorLocation`)))
    (bind _output_get (set `self.OverlappedActors` _outoverlappedactors))
    (for _array_element _output_get
      (`self.Burn` _array_element))
    (`KismetArrayLibrary.Array_Clear` _output_get)
    (else
      (`self.SetActorTickEnabled` false))))

(fn `ActivateFire`
  (params (InActor :type "/Game/Blueprints/Actor/Tree/BP_BaseTree Object Reference"))
  (bind _firesystem (`/Game/Blueprints/Actor/Tree/BP_BaseTree.FireSystem` InActor))
  (if (not (`ActorComponent.IsActive` _firesystem))
    (`ActorComponent.Activate` _firesystem true)
    (return)))

(fn `Burn`
  (params (InActor :type "Actor Object Reference"))
  (if (and (<= (`KismetMathLibrary.RandomFloatInRange` 0.0 1.0) (`self.ChanceToBurn`)) (not (`self.bIsBurning`)))
    (bind _asbp_base_tree (cast `/Game/Blueprints/Actor/Tree/BP_BaseTree` InActor))
    (set `/Game/Blueprints/Actor/Tree/BP_BaseTree.bIsBurning` true _asbp_base_tree)
    (`self.SetActorTickEnabled` _asbp_base_tree true)
    (`self.ActivateFire` _asbp_base_tree)
    (`self.SetLifeSpan` _asbp_base_tree (`KismetMathLibrary.RandomFloatInRange` 200.0 350.0))))

(fn `DeBurn`
  (set `self.bIsBurning` false)
  (`NiagaraFunctionLibrary.SpawnSystemAtLocation` "/Game/Resources/MegaMagicVFXBundle/VFX/MagicalExplosionsVFX/VFX/LightningExplosion/Systems/NS_HealBlastTiny.NS_HealBlastTiny" (`self.K2_GetActorLocation`))
  (`ActorComponent.Deactivate` (`self.FireSystem`))
  (`self.SetLifeSpan` 0.0))

(fn `UserConstructionScript`)