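; Game mode that tracks toxic terrain cleanup as the level's win condition.
; On BeginPlay it starts background music, gathers Toxic-tagged BP_BaseToxicTerrain actors and feeds the count to the overlay's toxicity widget via the Aura HUD.
; VerifyToxicity removes each destroyed terrain and refreshes the widget.
; When none remain, it destroys all BP_FireBase actors and shows the win screen.
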(event `self.ReceiveBeginPlay`
  (`GameplayStatics.PlaySound2D` "/Game/Assets/Music/sfx_AriaBackgroundMusic.sfx_AriaBackgroundMusic" 1.0 1.0 0.0 null null)
  (bind _outactors (`GameplayStatics.GetAllActorsOfClassWithTag` "/Game/Blueprints/Actor/Tree/BP_BaseToxicTerrain.BP_BaseToxicTerrain_C" "Toxic"))
  (bind _output_get (set `self.ToxicActors` _outactors))
  (bind _output_get_2 (set `self.MaxToxic` (`KismetArrayLibrary.Array_Length` _output_get)))
  (set `self.CurrentToxic` _output_get_2)
  (bind _asbp_aura_hud (cast `/Game/Blueprints/UI/HUD/BP_AuraHUD` (`PlayerController.GetHUD` (`GameplayStatics.GetPlayerController` 0))))
  (bind _returnvalue (`AuraHUD.GetOverlayWidget` _asbp_aura_hud))
  (bind _aswbp_overlay (cast `/Game/Blueprints/UI/Overlay/WBP_Overlay` _returnvalue))
  (bind _output_get_3 (set `self.WBPOverlay` _aswbp_overlay))
  (`/Game/Blueprints/UI/ToxicMeasure/WBP_Toxic.SetToxic` (`/Game/Blueprints/UI/Overlay/WBP_Overlay.WBP_Toxic` _output_get_3) (`self.CurrentToxic`) (`self.MaxToxic`)))

(event `VerifyToxicity`
  (params (InToxicDestroyed :type "/Game/Blueprints/Actor/Tree/BP_BaseToxicTerrain Object Reference"))
  (bind _toxicactors (`self.ToxicActors`))
  (bind _returnvalue (`KismetArrayLibrary.Array_Length` _toxicactors))
  (`KismetArrayLibrary.Array_RemoveItem` _toxicactors InToxicDestroyed)
  (set `self.CurrentToxic` _returnvalue)
  (`/Game/Blueprints/UI/ToxicMeasure/WBP_Toxic.SetToxic` (`/Game/Blueprints/UI/Overlay/WBP_Overlay.WBP_Toxic` (`self.WBPOverlay`)) (`self.CurrentToxic`) (`self.MaxToxic`))
  (if (== _returnvalue 0)
    (`self.ClearFire`)
    (bind _returnvalue_2 (`|CreateWidget` "/Game/Blueprints/UI/WinAria/WBP_CanvasWin.WBP_CanvasWin_C"))
    (`UserWidget.AddToViewport` _returnvalue_2 0)))

(fn `ClearFire`
  (bind _outactors (`GameplayStatics.GetAllActorsOfClass` "/Game/Blueprints/Actor/FireActor/BP_FireBase.BP_FireBase_C"))
  (for _array_element _outactors
    (`self.K2_DestroyActor` _array_element)))

(fn `UserConstructionScript`)