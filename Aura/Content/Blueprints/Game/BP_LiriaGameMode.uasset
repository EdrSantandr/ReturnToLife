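; Game mode for Liria that runs the in-game music and presents the win and lose end screens.
; BeginPlay spawns and plays the background music, keeping a reference to it.
; The ShowMessageYouWin and ShowMessageYouLose events stop that music, play their own sound, hide the cursor and switch player 0 to UI-only input.
; Each then creates its result widget, passes it the enemies-killed count and adds it to the viewport.
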(event `self.ReceiveBeginPlay`
  (bind _returnvalue (`GameplayStatics.SpawnSound2D` "/Game/Assets/Music/sfx_InGameBackgroundMusic.sfx_InGameBackgroundMusic" 1.0 1.0 0.0 null))
  (bind _output_get (set `self.InGameMusic` _returnvalue))
  (`AudioComponent.Play` _output_get 0.0))

(event `self.ShowMessageYouLose`
  (params (InEnemiesKilled :type Integer))
  (bind _returnvalue (`GameplayStatics.GetPlayerController` 0))
  (set `self.In Enemies Killed` InEnemiesKilled)
  (`AudioComponent.Stop` (`self.InGameMusic`))
  (`GameplayStatics.PlaySound2D` "/Game/Assets/Sounds/YouLose/sfx_YouLose.sfx_YouLose" 1.0 1.0 0.0 null null)
  (set `PlayerController.bShowMouseCursor` false _returnvalue)
  (`WidgetBlueprintLibrary.SetInputMode_UIOnlyEx` _returnvalue null)
  (bind _returnvalue_2 (`|CreateWidget` "/Game/Blueprints/UI/YouLose/WBP_YouLose.WBP_YouLose_C"))
  (`/Game/Blueprints/UI/YouLose/WBP_YouLose.OnShowWidget` _returnvalue_2 (`self.In Enemies Killed`))
  (`UserWidget.AddToViewport` _returnvalue_2 0))

(event `self.ShowMessageYouWin`
  (params (InEnemiesKilled :type Integer))
  (bind _returnvalue (`GameplayStatics.GetPlayerController` 0))
  (set `self.In Enemies Killed` InEnemiesKilled)
  (`AudioComponent.Stop` (`self.InGameMusic`))
  (`GameplayStatics.PlaySound2D` "/Game/Assets/Sounds/Music/sfx_MainMenu.sfx_MainMenu" 1.0 1.0 0.0 null null)
  (set `PlayerController.bShowMouseCursor` false _returnvalue)
  (`WidgetBlueprintLibrary.SetInputMode_UIOnlyEx` _returnvalue null)
  (bind _returnvalue_2 (`|CreateWidget` "/Game/Blueprints/UI/YouWin/WBP_YouWin.WBP_YouWin_C"))
  (`/Game/Blueprints/UI/YouWin/WBP_YouWin.OnShowWidget` _returnvalue_2 (`self.In Enemies Killed`))
  (`UserWidget.AddToViewport` _returnvalue_2 0))

(fn `UserConstructionScript`)