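; BP_AuraCharacter is the Aura character Blueprint, which plays a camera intro when play begins.
; BeginPlay sets UI-only input, zeroes walk speed and hides the HUD overlay, then after a delay a timeline lerps the camera from its initial location to its original position.
; On completion it restores the overlay, speed and game input.
; Separate events set shock and casting loop flags and update the FacingTarget motion warp location.
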(event `self.ReceiveBeginPlay`
  (bind _charactermovement (`self.CharacterMovement`))
  (`WidgetBlueprintLibrary.SetInputMode_UIOnlyEx` (`GameplayStatics.GetPlayerController` 0) null)
  (set `self.OriginalMaxSpeed` (`MovementComponent.GetMaxSpeed` _charactermovement))
  (set `CharacterMovementComponent.MaxWalkSpeed` 0.0 _charactermovement)
  (bind _asbp_aura_hud (cast `/Game/Blueprints/UI/HUD/BP_AuraHUD` (`PlayerController.GetHUD` (`GameplayStatics.GetPlayerController` 0))))
  (bind _returnvalue (`AuraHUD.GetOverlayWidget` _asbp_aura_hud))
  (set `self.OverlayWidget` _returnvalue)
  (`Widget.SetVisibility` _returnvalue "Hidden")
  (bind _returnvalue_2 (`self.GetCameraComponent`))
  (bind _output_get (set `self.CameraComponent` _returnvalue_2))
  (set `self.FinalCameraLocation` (`SceneComponent.K2_GetComponentLocation` _output_get))
  (`SceneComponent.K2_SetWorldLocation` _output_get (`self.InitialCameraLocation`) false false)
  (`KismetSystemLibrary.Delay` 1.0)
  (bind (_direction _location) (`Timeline|LocationTimeline` :!via `PlayFromStart`)
    (:`Update`
      (`SceneComponent.K2_SetWorldLocation` (`self.CameraComponent`) (`KismetMathLibrary.VLerp` (`self.InitialCameraLocation`) (`self.FinalCameraLocation`) _location) false false))
    (:`Finished`
      (`SceneComponent.K2_SetWorldLocation` (`self.CameraComponent`) (`self.FinalCameraLocation`) false false)
      (set `Widget.Visibility` "Visible" (`self.OverlayWidget`))
      (set `CharacterMovementComponent.MaxWalkSpeed` (`self.OriginalMaxSpeed`) (`self.CharacterMovement`))
      (`WidgetBlueprintLibrary.SetInputMode_GameOnly` (`GameplayStatics.GetPlayerController` 0)))))

(event `CombatInterface.SetInShockLoop`
  (params (bInLoop :type Boolean))
  (set `self.InShockLoop` bInLoop))

(event `CombatInterface.SetIsCastingLoop`
  (params (bInCastingLoop :type Boolean))
  (set `self.InCastingLoop` bInCastingLoop))

(event `CombatInterface.UpdateFacingTarget`
  (params (Target :type "Vector Structure (by ref)"))
  (`MotionWarpingComponent.AddOrUpdateWarpTargetFromLocation` (`self.MotionWarping`) "FacingTarget" Target))

(fn `UserConstructionScript`)